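; GM_AITTS, apparently a game mode, is a prototype for AI text-to-speech whose speech and AI parts are disconnected.
; On BeginPlay it creates players for two camera Level Sequences, without starting playback.
; Unwired chains would speak test text on a TeaPotVoice channel through the TextToSpeech subsystem and call OpenAI GPT-3 with an empty prompt.
; The GPT-3 chain contains a hardcoded API key.
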(event EventBeginPlay
  (Sequencer|Player|CreateLevelSequencePlayer "/Game/CameraSequenceA.CameraSequenceA")
  (Sequencer|Player|CreateLevelSequencePlayer "/Game/CameraSequenceB.CameraSequenceB"))

(event EventTick
  (params (DeltaSeconds :type Float%20%28single-precision%29)))

(fn ConstructionScript)